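; BP_Planet is a planet actor that supplies gravity information to ships entering its sphere of influence.
; At BeginPlay it builds an SPlanetInfo struct from its location, sphere radius and Strength value.
; When a BP_Ship overlaps the sphere, the planet passes that info to the ship and enables its gravity flag.
; Ending the overlap turns the flag off, leaving the pull itself outside this Blueprint.
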(event OnComponentBeginOverlap(Sphere)
  (params (OverlappedComponent :type Primitive%20Component%20Object%20Reference) (OtherActor :type Actor%20Object%20Reference) (OtherComp :type Primitive%20Component%20Object%20Reference) (OtherBodyIndex :type Integer) (bFromSweep :type Boolean) (SweepResult :type Hit%20Result%20Structure%20%28by%20ref%29))
  (bind _asbp_ship (Utilities|Casting|CastToBP_Ship OtherActor))
  (Variables|/Game/Player/BP_Ship.BP_Ship_C|SetCurrentPlanetInfo _asbp_ship (Variables|Default|GetPlanetInfo))
  (Variables|/Game/Player/BP_Ship.BP_Ship_C|SetGravityActive _asbp_ship true))

(event OnComponentEndOverlap(Sphere)
  (params (OverlappedComponent :type Primitive%20Component%20Object%20Reference) (OtherActor :type Actor%20Object%20Reference) (OtherComp :type Primitive%20Component%20Object%20Reference) (OtherBodyIndex :type Integer))
  (bind _asbp_ship (Utilities|Casting|CastToBP_Ship OtherActor))
  (Variables|/Game/Player/BP_Ship.BP_Ship_C|SetGravityActive _asbp_ship false))

(event EventBeginPlay
  (Variables|Default|SetPlanetInfo (Utilities|Struct|MakeS_PlanetInfo (Transformation|GetActorLocation) (Variables|/Script/Engine.SphereComponent|GetSphereRadius (Variables|Default|GetSphere)) (Variables|Default|GetStrength))))

(fn ConstructionScript)