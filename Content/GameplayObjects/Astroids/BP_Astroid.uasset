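; BP_Astroid is a mineable asteroid actor that is destroyed once its ore runs out.
; An AstroidonMine event subtracts the given Power from RemainingOre, prints the remaining amount, and destroys the actor at zero or below.
; A ReturnActor function returns a reference to the asteroid itself.
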(event EventAstroidonMine
  (params (Power :type Float%20%28double-precision%29))
  (bind _output_get (Variables|Default|SetRemainingOre (- (Variables|Default|GetRemainingOre) Power)))
  (Development|PrintString (Utilities|String|ToString(Float) _output_get))
  (if (<= (Variables|Default|GetRemainingOre) 0.0)
    (Actor|DestroyActor)))

(fn ConstructionScript)

(fn ReturnActor
  (return self))