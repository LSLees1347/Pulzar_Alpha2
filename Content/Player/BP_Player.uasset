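; Player Blueprint that moves a Point component with the mouse and offers a toggleable ball camera.
; Mouse input offsets Point along its local Y and Z axes.
; BeginPlay caches the first BP_Ball found, and IA_CamLock flips BallCam on and off.
; Tick sets control rotation to the camera-to-ball look-at pitch while BallCam is on, otherwise zero, with yaw and roll always zero.
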(event Input|EnhancedActionEvents|EnhancedInputActionIA_Mouse
  (params (ActionValue :type Vector%202D%20Structure) (ElapsedSeconds :type Float%20%28double-precision%29) (TriggeredSeconds :type Float%20%28double-precision%29) (InputAction :type Input%20Action%20Object%20Reference :default "/Game/Input/IA_Mouse.IA_Mouse"))
  (Transformation|AddLocalOffset (Variables|Default|GetPoint) (Math|Vector|MakeVector 0.0 (* (.x ActionValue) 2.0) (* (.y ActionValue) 2.0)) false false))

(event Input|EnhancedActionEvents|EnhancedInputActionIA_CamLock
  (params (ActionValue :type Boolean) (ElapsedSeconds :type Float%20%28double-precision%29) (TriggeredSeconds :type Float%20%28double-precision%29) (InputAction :type Input%20Action%20Object%20Reference :default "/Game/Input/IA_CamLock.IA_CamLock"))
  (:Started
    (Utilities|FlowControl|FlipFlop
      (:A
        (Variables|Default|SetBallCam true)
        (Development|PrintString "BallCam"))
      (:B
        (Variables|Default|SetBallCam false)))))

(event EventBeginPlay
  (bind _outactors (Actor|GetAllActorsOfClass "/Game/Player/BP_Ball.BP_Ball_C"))
  (Variables|Default|SetBP_Ball (Utilities|Array|Get(acopy) _outactors)))

(event EventTick
  (params (DeltaSeconds :type Float%20%28single-precision%29))
  (bind _returnvalue (Pawn|GetController))
  (if (Variables|Default|GetBallCam)
    (Variables|Default|GetBP_Ball
      (:then
        (Pawn|SetControlRotation _returnvalue (Math|Rotator|MakeRotator 0.0 (.pitch (Math|Rotator|FindLookatRotation (Transformation|GetWorldLocation (Variables|Default|GetCamera)) (Transformation|GetActorLocation (Variables|Default|GetBP_Ball)))) 0.0)))
      (:else
        (Development|PrintString "invalid")))
    (else
      (Pawn|SetControlRotation _returnvalue (Math|Rotator|MakeRotator 0.0 0.0 0.0)))))

(fn ConstructionScript)