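; Player ship pawn with a flipbook sprite that thrusts, strafes, brakes, boosts and fires through Enhanced Input.
; FloatingPawnMovement drives motion, tuned from variables at construction; braking temporarily raises deceleration, and thrust swaps the flipbook.
; Turnto smoothly yaws the ship toward a supplied target, and firing spawns BP_Bullet with the ship's transform and velocity.
; Boost plays a timeline that ramps TurningBoost, locked against retriggering until it finishes and zeroes the value.
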(event Input|EnhancedActionEvents|EnhancedInputActionIA_Thrust
  (params (ActionValue :type Float%20%28double-precision%29) (ElapsedSeconds :type Float%20%28double-precision%29) (TriggeredSeconds :type Float%20%28double-precision%29) (InputAction :type Input%20Action%20Object%20Reference :default "/Game/Input/IA_Thrust.IA_Thrust"))
  (:Triggered
    (Pawn|Input|AddMovementInput (Transformation|GetActorForwardVector) 1.0 false)
    (Sprite|SetFlipbook (Variables|Default|GetPaperFlipbook) "/Game/Player/Art/Test/BattleShipThrust_Flipbook.BattleShipThrust_Flipbook"))
  (:Completed
    (Sprite|SetFlipbook (Variables|Default|GetPaperFlipbook) "/Game/Player/Art/Test/BattleShip_Flipbook.BattleShip_Flipbook")))

(event Input|EnhancedActionEvents|EnhancedInputActionIA_Brake
  (params (ActionValue :type Boolean) (ElapsedSeconds :type Float%20%28double-precision%29) (TriggeredSeconds :type Float%20%28double-precision%29) (InputAction :type Input%20Action%20Object%20Reference :default "/Game/Input/IA_Brake.IA_Brake"))
  (bind _floatingpawnmovement (Variables|Default|GetFloatingPawnMovement))
  (:Started
    (Variables|/Script/Engine.FloatingPawnMovement|SetDeceleration _floatingpawnmovement 5e+02))
  (:Canceled
    (Variables|/Script/Engine.FloatingPawnMovement|SetDeceleration _floatingpawnmovement 25.0 :!label _label))
  (:Completed
    (goto _label)))

(event Input|EnhancedActionEvents|EnhancedInputActionIA_Fire
  (params (ActionValue :type Boolean) (ElapsedSeconds :type Float%20%28double-precision%29) (TriggeredSeconds :type Float%20%28double-precision%29) (InputAction :type Input%20Action%20Object%20Reference :default "/Game/Input/IA_Fire.IA_Fire"))
  (bind _returnvalue (Transformation|GetActorTransform))
  (:Started
    (Game|SpawnActorfromClass "/Game/Player/BP_Bullet.BP_Bullet_C" (Math|Transform|MakeTransform (Math|Vector|MakeVector (.x (.location _returnvalue)) (.y (.location _returnvalue)) 0.0) (Math|Rotator|MakeRotator 0.0 0.0 (.yaw (.rotation _returnvalue))) "1.000000,1.000000,1.000000") "Undefined" "MultiplyWithRoot" 0 (Transformation|GetVelocity) 0)))

(event Input|EnhancedActionEvents|EnhancedInputActionIA_Boost
  (params (ActionValue :type Boolean) (ElapsedSeconds :type Float%20%28double-precision%29) (TriggeredSeconds :type Float%20%28double-precision%29) (InputAction :type Input%20Action%20Object%20Reference :default "/Game/Input/IA_Boost.IA_Boost"))
  (bind _floatingpawnmovement (Variables|Default|GetFloatingPawnMovement))
  (:Started
    (if (Variables|Default|GetCanTB)
      (Variables|Default|SetCanTB false)
      (bind _newtrack_0 (Timeline|TB_trans PlayFromStart)
        (:Update
          (Variables|/Script/Engine.FloatingPawnMovement|SetTurningBoost _floatingpawnmovement (Math|Float|Lerp 0.0 25.0 _newtrack_0)))
        (:Finished
          (Variables|Default|SetCanTB true)
          (Variables|/Script/Engine.FloatingPawnMovement|SetTurningBoost _floatingpawnmovement 0.0))))))

(event Input|EnhancedActionEvents|EnhancedInputActionIA_Left
  (params (ActionValue :type Boolean) (ElapsedSeconds :type Float%20%28double-precision%29) (TriggeredSeconds :type Float%20%28double-precision%29) (InputAction :type Input%20Action%20Object%20Reference :default "/Game/Input/IA_Left.IA_Left"))
  (Pawn|Input|AddMovementInput (Math|Vector|NegateVector (Transformation|GetActorRightVector)) 0.5 false))

(event Input|EnhancedActionEvents|EnhancedInputActionIA_Right
  (params (ActionValue :type Boolean) (ElapsedSeconds :type Float%20%28double-precision%29) (TriggeredSeconds :type Float%20%28double-precision%29) (InputAction :type Input%20Action%20Object%20Reference :default "/Game/Input/IA_Right.IA_Right"))
  (Pawn|Input|AddMovementInput (Transformation|GetActorRightVector) 0.5 false))

(event EventTurnto
  (params (Target :type Vector :default "0, 0, 0"))
  (bind _returnvalue (Transformation|GetActorLocation))
  (Transformation|SetActorRotation (Math|Interpolation|RInterpTo (Transformation|GetActorRotation) (Math|Rotator|FindLookatRotation (Math|Vector|MakeVector (.x _returnvalue) (.y _returnvalue) 0.0) (Math|Vector|MakeVector (.x Target) (.y Target) 0.0)) (Utilities|Time|GetWorldDeltaSeconds) 8.0)))

(fn ConstructionScript
  (bind _floatingpawnmovement (Variables|Default|GetFloatingPawnMovement))
  (Variables|/Script/Engine.FloatingPawnMovement|SetMaxSpeed _floatingpawnmovement (Variables|Default|GetMaxSpeed))
  (Variables|/Script/Engine.FloatingPawnMovement|SetAcceleration _floatingpawnmovement (Variables|Default|GetAcceleration))
  (Variables|/Script/Engine.FloatingPawnMovement|SetDeceleration _floatingpawnmovement (Variables|Default|GetDeceleration))
  (Variables|/Script/Engine.FloatingPawnMovement|SetTurningBoost _floatingpawnmovement (Variables|Default|GetTurnBoost)))