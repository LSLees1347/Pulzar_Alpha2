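; BP_Miner is a player-controlled miner that thrusts around and mines asteroids with a laser.
; Primary input picks a target and, if it is within range, spawns a Niagara beam with its endpoint set once at spawn.
; A Delay loop repeats range checks and mining messages, removing the beam when a hit leaves the target invalid.
; Thrust input calls ThrustMovement and toggles the thruster effect.
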(event Input|EnhancedActionEvents|EnhancedInputActionIA_Thrust
  (params (ActionValue :type Boolean) (ElapsedSeconds :type Float%20%28double-precision%29) (TriggeredSeconds :type Float%20%28double-precision%29) (InputAction :type Input%20Action%20Object%20Reference :default "/Game/Input/IA_Thrust.IA_Thrust"))
  (bind _thruster1 (Variables|Default|GetThruster1))
  (:Triggered
    (CallFunction|ThrustMovement))
  (:Started
    (Components|Activation|SetActive _thruster1 true false))
  (:Completed
    (Components|Activation|SetActive _thruster1 false false)))

(event Input|EnhancedActionEvents|EnhancedInputActionIA_Primary
  (params (ActionValue :type Boolean) (ElapsedSeconds :type Float%20%28double-precision%29) (TriggeredSeconds :type Float%20%28double-precision%29) (InputAction :type Input%20Action%20Object%20Reference :default "/Game/Input/IA_Primary.IA_Primary"))
  (bind _activetarget (Variables|Default|GetActiveTarget))
  (bind _returnvalue (Transformation|GetActorLocation _activetarget))
  (:Started
    (if (not (Variables|Default|GetIsMining))
      (CallFunction|ChangeTarget)
      (Variables|Default|GetActiveTarget :!label _label
        (:then
          (if (< (Transformation|GetDistanceTo self (Variables|Default|GetActiveTarget)) (Variables|Default|GetLaserRange))
            (Variables|Default|SetIsMining true)
            (Variables|Default|GetActiveLaser
              (:then
                _)
              (:else
                (bind _returnvalue_2 (Niagara|SpawnSystemAttached "/Game/VFX/NS_Laser.NS_Laser" (Variables|Default|GetFirePoint) "None" "0, 0, 0" "0, 0, 0" "KeepRelativeOffset" true))
                (bind _output_get (Variables|Default|SetActiveLaser _returnvalue_2))
                (Class|NiagaraComponent|SetVariablePosition _output_get "Beam End" (Math|Vector|MakeVector (.x _returnvalue) (.y _returnvalue) 0.0))))
            (Class|BPIActors|AstroidonMine(Message) (Variables|Default|GetActiveTarget) (Variables|Default|GetLaserPower))
            (Variables|Default|GetActiveTarget
              (:then
                (Utilities|FlowControl|Delay (Variables|Default|GetLaserCooldown))
                (goto _label))
              (:else
                (Components|DestroyComponent (Variables|Default|GetActiveLaser))
                (Variables|Default|SetIsMining false)))
            (else
              (Development|PrintString "too far"))))
        (:else
          (Development|PrintString "no target"))))))

(event EventBeginPlay
  (|CallParentFunction))

(event EventTick
  (params (DeltaSeconds :type Float%20%28single-precision%29))
  (|CallParentFunction DeltaSeconds))

(fn ConstructionScript
  (|CallParentFunction))